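; Knight (Rycerz) unit of the Zakon faction, with a passive shield (Tarcza) that periodically blocks incoming attacks.
; When the knight is the victim in the pre-attack stage, the shield's action counter increments and, on reset, stops the attack sequence.
; TargetFractionCheck intersects the knight's gameplay tags with another actor's and returns whether any shared tag falls under Fractions.
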(event AttackStageExecution(Passive_Tarcza)
  (params (AttackSequence :type Attack%20Sequence%20Object%20Reference))
  (Class|ActionCounterComponent|IncrementandCheckforReset (Variables|Default|GetActionCounter_Tarcza)
    (:True
      (Class|AttackSequence|StopExecution AttackSequence))))

(fn ConstructionScript)

(fn TargetFractionCheck
  (params (OtherActor :type Actor%20Object%20Reference))
  (Utilities|FlowControl|Sequence
    (:then_0
      (bind _tagcontainer (GameplayTags|GetOwnedGameplayTags OtherActor :!class /Script/GameplayTags.GameplayTagAssetInterface))
      (for _array_element (GameplayTags|BreakGameplayTagContainer _tagcontainer)
        (if (GameplayTags|HasTag (GameplayTags|GetOwnedGameplayTags (Variables|Default|GetAbilitySystemComponent) :!class /Script/GameplayTags.GameplayTagAssetInterface) _array_element true)
          (GameplayTags|AddGameplayTag (LocalVariables|GetMatchingTags) _array_element :!class /Script/GameplayTags.BlueprintGameplayTagLibrary))))
    (:then_1
      (return (GameplayTags|HasTag (LocalVariables|GetMatchingTags) "(TagName=\"Fractions\")")))))